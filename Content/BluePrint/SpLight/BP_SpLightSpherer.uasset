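; BP_SpLightSpherer is a placeable spherical light source that passes strength, hardness, radius and offset to its SpLightComponent and exposes them through a getter.
; The construction script sizes the influence sphere and shadow box, then scales and offsets a range-preview plane.
; A dynamic material on that plane draws the inner and outer range, bounded by the box extents relative to the offset.
; The plane is optionally shown in game, refreshing those bounds each tick.
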(event EventBeginPlay
  (Development|SetHiddeninGame (Variables|Default|GetLightInfluenceRangePlane) (not (Variables|SpLight|GetViewInGameLightInfluenceRange)) false))

(event EventTick
  (params (DeltaSeconds :type Float%20%28single-precision%29))
  (Transformation|SetRelativeLocation (Variables|Default|GetLightInfluenceRangePlane) (Variables|SpLight|GetOffset) false false)
  (if (not (Variables|/Script/Engine.SceneComponent|GetbHiddenInGame (Variables|Default|GetLightInfluenceRangePlane)))
    (CallFunction|UpdateMaterialColor)))

(fn ConstructionScript
  (bind _radius (Variables|SpLight|GetRadius))
  (bind _returnvalue (/ _radius 5e+01))
  (Utilities|FlowControl|Sequence
    (:then_0
      (Components|Sphere|SetSphereRadius (Variables|Default|GetLightSourceInfluenceSphere) _radius false))
    (:then_1
      (Components|Box|SetBoxExtent (Variables|Default|GetShadowEffectiveBox) (Variables|SpLight|GetRightRangeBox) false)
      (Transformation|SetRelativeScale3D (Variables|Default|GetLightInfluenceRangePlane) (Math|Vector|MakeVector _returnvalue _returnvalue _returnvalue))
      (SpLight|SetandUpdateLightComp (Variables|SpLight|GetStrength) (Variables|SpLight|GetHardness) (Variables|SpLight|GetRadius) (Variables|SpLight|GetOffset))
      (Transformation|SetRelativeLocation (Variables|Default|GetLightInfluenceRangePlane) (Variables|SpLight|GetOffset) false false))
    (:then_2
      (bind _returnvalue_2 (Rendering|Material|CreateDynamicMaterialInstance (Variables|Default|GetLightInfluenceRangePlane) 0 0 "None" :!class /Script/Engine.PrimitiveComponent))
      (Variables|Default|SetMID_PlaneColor _returnvalue_2)
      (Rendering|Material|SetScalarParameterValue _returnvalue_2 "Radius" (Variables|SpLight|GetRadius) :!class /Script/Engine.MaterialInstanceDynamic)
      (CallFunction|UpdateMaterialColor)
      (Rendering|Material|SetScalarParameterValue _returnvalue_2 "Hardness" (Variables|SpLight|GetHardness) :!class /Script/Engine.MaterialInstanceDynamic)
      (Utilities|FlowControl|Sequence
        (:then_0
          (Rendering|Material|SetVectorParameterValue _returnvalue_2 "ColorRangeIn" (Variables|SpLight|GetLightRangeIn) :!class /Script/Engine.MaterialInstanceDynamic)
          (Rendering|Material|SetVectorParameterValue _returnvalue_2 "ColorRangeOut" (Variables|SpLight|GetLightRangeOut) :!class /Script/Engine.MaterialInstanceDynamic))
        (:then_1
          (Rendering|Material|SetScalarParameterValue _returnvalue_2 "OpacityRangeIn" (Variables|SpLight|GetOpacityRangeIn) :!class /Script/Engine.MaterialInstanceDynamic)
          (Rendering|Material|SetScalarParameterValue _returnvalue_2 "OpacityRangeOut" (Variables|SpLight|GetOpacityRangeOut) :!class /Script/Engine.MaterialInstanceDynamic))))))

(fn GetLightParameters
  (return (Variables|SpLight|GetStrength) (Variables|SpLight|GetHardness) (Variables|SpLight|GetRadius) (Default|GetLightLocation (Variables|Default|GetSpLightComponent))))

(fn SetandUpdateLightComp
  (params (Strength :type Float%20%28double-precision%29) (Hardness :type Float%20%28double-precision%29) (Radius :type Float%20%28double-precision%29) (Offset :type Vector))
  (Default|SetandUpdateLight (Variables|Default|GetSpLightComponent) Strength Hardness Radius Offset))

(fn UpdateLightComp
  (SpLight|SetandUpdateLightComp (Variables|SpLight|GetStrength) (Variables|SpLight|GetHardness) (Variables|SpLight|GetRadius) (Variables|SpLight|GetOffset)))

(fn UpdateMaterialColor
  (bind _mid_planecolor (Variables|Default|GetMID_PlaneColor))
  (bind _rightrangebox (Variables|SpLight|GetRightRangeBox))
  (bind _offset (Variables|SpLight|GetOffset))
  (bind _rightrangebox_2 (Variables|SpLight|GetRightRangeBox))
  (bind _offset_2 (Variables|SpLight|GetOffset))
  (bind _returnvalue (* _rightrangebox 1.0))
  (bind _returnvalue_2 (* _rightrangebox_2 -1.0))
  (bind _returnvalue_3 (- _returnvalue_2 _offset_2))
  (bind _returnvalue_4 (- _returnvalue _offset))
  (bind (_x _y _z) (Math|Vector|BreakVector _returnvalue_4))
  (bind (_x_2 _y_2 _z_2) (Math|Vector|BreakVector _returnvalue_3))
  (Rendering|Material|SetScalarParameterValue _mid_planecolor "RangeXLeft" _y_2 :!class /Script/Engine.MaterialInstanceDynamic)
  (Rendering|Material|SetScalarParameterValue _mid_planecolor "RangeYBottom" _z_2 :!class /Script/Engine.MaterialInstanceDynamic)
  (Rendering|Material|SetScalarParameterValue _mid_planecolor "RangeXRIght" _y :!class /Script/Engine.MaterialInstanceDynamic)
  (Rendering|Material|SetScalarParameterValue _mid_planecolor "RangeYTop" _z :!class /Script/Engine.MaterialInstanceDynamic))