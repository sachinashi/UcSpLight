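; Component that receives custom sprite lighting by writing light and look parameters into a sprite dynamic material instance.
; Init stores the material and an optional self light, which it updates every Tick and whose change dispatcher feeds the SelfLight parameters, matching how placed lights work.
; Separate setters drive or reset a sphere light from a given light component, and adjust overall contrast and strength, color shift, color correction and normal strengths.
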(event Custom|ChangeSpLightSelf
  (params (Strength :type Float%20%28double-precision%29) (Hardness :type Float%20%28double-precision%29) (Radius :type Float%20%28double-precision%29) (WorldLocation :type Vector))
  (bind _ucsplightself (Variables|SpLight|Self|GetUcSpLightSelf))
  ;[1 1 1] セルフライトの処理
  (Utilities|IsValid _ucsplightself
    (:Is%20Valid
      (SpLight|SetLightSelf _ucsplightself))))

(event EventBeginPlay)

(event EventTick
  (params (DeltaSeconds :type Float%20%28single-precision%29))
  (bind _ucsplightself (Variables|SpLight|Self|GetUcSpLightSelf))
  ;[1 1 1] セルフライトの処理
  (Utilities|IsValid _ucsplightself
    (:Is%20Valid
      (Default|UpdateLight _ucsplightself))))

(fn Init
  (params (MIDUcSpLight :type Material%20Instance%20Dynamic%20Object%20Reference) (SelfLight :type BP%20Sp%20Light%20Component%20Object%20Reference))
  (Variables|SpLight|SetMIDUcSpLight MIDUcSpLight) ; スプライト管理マテリアルの初期化
  ;[1 1 1] セルフライトの初期化
  (bind _output_get (Variables|SpLight|Self|SetUcSpLightSelf SelfLight))
  (Utilities|IsValid _output_get
    (:Is%20Valid
      (EventDispatchers|BindEventtoOnChangeLightParam _output_get (EventDispatchers|CreateEvent :!event Custom|ChangeSpLightSelf)))
    (:Is%20Not%20Valid
      _))
  (return (Utilities|IsValid (Variables|SpLight|GetMIDUcSpLight))))

(fn SetLightSphere
  (params (UcSpLightComp :type BP%20Sp%20Light%20Component%20Object%20Reference))
  (SpLight|SetLightSphereParam (Variables|/UcSpLight/BluePrint/Component/BP_SpLightComponent.BP_SpLightComponent_C|GetStrength UcSpLightComp) (Variables|/UcSpLight/BluePrint/Component/BP_SpLightComponent.BP_SpLightComponent_C|GetHardness UcSpLightComp) (Variables|/UcSpLight/BluePrint/Component/BP_SpLightComponent.BP_SpLightComponent_C|GetRadius UcSpLightComp) (Default|GetLightLocation UcSpLightComp))
  (return))

(fn SetLightSphereParam
  (params (Strength :type Float%20%28double-precision%29) (Hardness :type Float%20%28double-precision%29) (Radius :type Float%20%28double-precision%29) (Location :type Vector))
  (bind _miducsplight (Variables|SpLight|GetMIDUcSpLight))
  (Utilities|IsValid _miducsplight
    (:Is%20Valid
      (Rendering|Material|SetScalarParameterValue _miducsplight "SphereLightStrength" Strength :!class /Script/Engine.MaterialInstanceDynamic)
      (Rendering|Material|SetScalarParameterValue _miducsplight "SphereLightEdgeHardness" Hardness :!class /Script/Engine.MaterialInstanceDynamic)
      (Rendering|Material|SetScalarParameterValue _miducsplight "SphereLightRadius" Radius :!class /Script/Engine.MaterialInstanceDynamic)
      (Rendering|Material|SetVectorParameterValue _miducsplight "SphereLightPosition" (Math|Conversions|ToLinearColor(Vector) Location) :!class /Script/Engine.MaterialInstanceDynamic))
    (:Is%20Not%20Valid
      _))
  (return))

(fn SetLightSelf
  (params (UcSpLightComp :type BP%20Sp%20Light%20Component%20Object%20Reference))
  (SpLight|SetLightSelfParam (Variables|/UcSpLight/BluePrint/Component/BP_SpLightComponent.BP_SpLightComponent_C|GetStrength UcSpLightComp) (Variables|/UcSpLight/BluePrint/Component/BP_SpLightComponent.BP_SpLightComponent_C|GetHardness UcSpLightComp) (Variables|/UcSpLight/BluePrint/Component/BP_SpLightComponent.BP_SpLightComponent_C|GetRadius UcSpLightComp) (Default|GetLightLocation UcSpLightComp))
  (return))

(fn SetLightSelfParam
  (params (Strength :type Float%20%28double-precision%29) (Hardness :type Float%20%28double-precision%29) (Radius :type Float%20%28double-precision%29) (Location :type Vector))
  (bind _miducsplight (Variables|SpLight|GetMIDUcSpLight))
  (Utilities|IsValid _miducsplight
    (:Is%20Valid
      (Rendering|Material|SetScalarParameterValue _miducsplight "SelfLightStrength" Strength :!class /Script/Engine.MaterialInstanceDynamic)
      (Rendering|Material|SetScalarParameterValue _miducsplight "SelfLightEdgeHardness" Hardness :!class /Script/Engine.MaterialInstanceDynamic)
      (Rendering|Material|SetScalarParameterValue _miducsplight "SelfLightRadius" Radius :!class /Script/Engine.MaterialInstanceDynamic)
      (Rendering|Material|SetVectorParameterValue _miducsplight "SelfLightPosition" (Math|Conversions|ToLinearColor(Vector) Location) :!class /Script/Engine.MaterialInstanceDynamic))
    (:Is%20Not%20Valid
      _))
  (return))

(fn ResetLightSphere
  (SpLight|SetLightSphereParam 0.0 0.0 0.0 (Utilities|InitialLightLocationOffset)))

(fn SetOverall
  (params (Contrast :type Float%20%28single-precision%29) (Strenght :type Float%20%28single-precision%29))
  (bind _miducsplight (Variables|SpLight|GetMIDUcSpLight))
  (Rendering|Material|SetScalarParameterValue _miducsplight "OvreallContrast" Contrast :!class /Script/Engine.MaterialInstanceDynamic)
  (Rendering|Material|SetScalarParameterValue _miducsplight "OvreallStrenght" Strenght :!class /Script/Engine.MaterialInstanceDynamic))

(fn SetColorType
  (params (ShiftAmount :type Float%20%28single-precision%29))
  (Rendering|Material|SetScalarParameterValue (Variables|SpLight|GetMIDUcSpLight) "ColorTypeShiftAmount" ShiftAmount :!class /Script/Engine.MaterialInstanceDynamic))

(fn SetColorCorrection
  (params (ColorCorrection :type Linear%20Color%20Structure))
  (Rendering|Material|SetVectorParameterValue (Variables|SpLight|GetMIDUcSpLight) "ColorCorrection" ColorCorrection :!class /Script/Engine.MaterialInstanceDynamic))

(fn SetNormal
  (params (NormalStrength :type Float%20%28single-precision%29) (NormalStrengthR :type Float%20%28double-precision%29) (NormalStrengthG :type Float%20%28double-precision%29) (NormalStrengthB :type Float%20%28double-precision%29))
  (bind _miducsplight (Variables|SpLight|GetMIDUcSpLight))
  (Rendering|Material|SetScalarParameterValue _miducsplight "NormalStrength" NormalStrength :!class /Script/Engine.MaterialInstanceDynamic)
  (Rendering|Material|SetScalarParameterValue _miducsplight "NormalStrengthR" NormalStrengthR :!class /Script/Engine.MaterialInstanceDynamic)
  (Rendering|Material|SetScalarParameterValue _miducsplight "NormalStrengthG" NormalStrengthG :!class /Script/Engine.MaterialInstanceDynamic)
  (Rendering|Material|SetScalarParameterValue _miducsplight "NormalStrengthB" NormalStrengthB :!class /Script/Engine.MaterialInstanceDynamic))