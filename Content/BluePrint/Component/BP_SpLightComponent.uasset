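; BP_SpLightComponent is a light component that holds strength, hardness, radius and offset, and reports changes to them.
; SetAndUpdateLight stores the values, then UpdateLight passes strength, hardness, radius and light location to CallOnChangeLightParam.
; The light location is the component's world location plus the unrotated offset.
; BeginPlay and Tick are empty, and an unconnected debug print shows owner, component name and light location.
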(event EventBeginPlay)

(event EventTick
  (params (DeltaSeconds :type Float%20%28single-precision%29)))

(fn SetandUpdateLight
  (params (Strength :type Float%20%28double-precision%29) (Hardness :type Float%20%28double-precision%29) (Radius :type Float%20%28double-precision%29) (Offset :type Vector))
  (Variables|SpLight|SetStrength Strength)
  (Variables|SpLight|SetHardness Hardness)
  (Variables|SpLight|SetRadius Radius)
  (Variables|SpLight|SetOffset Offset)
  (SpLight|UpdateLight))

(fn UpdateLight
  (Default|CallOnChangeLightParam (Variables|SpLight|GetStrength) (Variables|SpLight|GetHardness) (Variables|SpLight|GetRadius) (SpLight|GetLightLocation)))

(fn GetLightLocation
  (return (+ (Variables|SpLight|GetOffset) (Transformation|GetWorldLocation self))))