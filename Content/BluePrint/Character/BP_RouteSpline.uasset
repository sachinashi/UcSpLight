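; Route spline actor that hands its spline and an XY-reverse flag to overlapping BPI_SpLightRouteSpline actors as their rotate spline.
; Boxes at both ends assign the spline on entry and remove it when the actor exits not heading inward, judged by dot product.
; Leaving the enclosing capsule also removes it.
; The construction script aligns boxes to endpoint tangents and fits the capsule from point centroid, spread, box extents and buffer.
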(event OnComponentBeginOverlap(BoxStart)
  (params (OverlappedComponent :type Primitive%20Component%20Object%20Reference) (OtherActor :type Actor%20Object%20Reference) (OtherComp :type Primitive%20Component%20Object%20Reference) (OtherBodyIndex :type Integer) (bFromSweep :type Boolean) (SweepResult :type Hit%20Result%20Structure%20%28by%20ref%29))
  (Utilities|DoseImplementBpiSpLightRouteSpline OtherActor
    (:Then
      (Class|BPISpLightRouteSpline|SetRotateSpline(Message) OtherActor (Utilities|ResolveSoftReference (Variables|Default|GetSpline)) (Variables|スプライン|GetUseReverseDirectionXY)))))

(event OnComponentEndOverlap(BoxStart)
  (params (OverlappedComponent :type Primitive%20Component%20Object%20Reference) (OtherActor :type Actor%20Object%20Reference) (OtherComp :type Primitive%20Component%20Object%20Reference) (OtherBodyIndex :type Integer))
  (Utilities|DoseImplementBpiSpLightRouteSpline OtherActor
    (:Then
      (bind _direction (Class|BPISpLightRouteSpline|GetDirectionVector(Message) OtherActor))
      (if (<= (Math|Vector|DotProduct (Math|Vector|GetForwardVector (Variables|Default|GetBoxStart)) _direction) 0.05)
        (Class|BPISpLightRouteSpline|RemoveRotateSpline(Message) OtherActor (Utilities|ResolveSoftReference (Variables|Default|GetSpline)))))))

(event OnComponentBeginOverlap(BoxEnd)
  (params (OverlappedComponent :type Primitive%20Component%20Object%20Reference) (OtherActor :type Actor%20Object%20Reference) (OtherComp :type Primitive%20Component%20Object%20Reference) (OtherBodyIndex :type Integer) (bFromSweep :type Boolean) (SweepResult :type Hit%20Result%20Structure%20%28by%20ref%29))
  (Utilities|DoseImplementBpiSpLightRouteSpline OtherActor
    (:Then
      (Class|BPISpLightRouteSpline|SetRotateSpline(Message) OtherActor (Utilities|ResolveSoftReference (Variables|Default|GetSpline)) (Variables|スプライン|GetUseReverseDirectionXY)))))

(event OnComponentEndOverlap(BoxEnd)
  (params (OverlappedComponent :type Primitive%20Component%20Object%20Reference) (OtherActor :type Actor%20Object%20Reference) (OtherComp :type Primitive%20Component%20Object%20Reference) (OtherBodyIndex :type Integer))
  (Utilities|DoseImplementBpiSpLightRouteSpline OtherActor
    (:Then
      (bind _direction (Class|BPISpLightRouteSpline|GetDirectionVector(Message) OtherActor))
      (if (<= (Math|Vector|DotProduct (Math|Vector|GetForwardVector (Variables|Default|GetBoxEnd)) _direction) 0.05)
        (Class|BPISpLightRouteSpline|RemoveRotateSpline(Message) OtherActor (Utilities|ResolveSoftReference (Variables|Default|GetSpline)))))))

(event OnComponentEndOverlap(ValidRangeCapsule)
  (params (OverlappedComponent :type Primitive%20Component%20Object%20Reference) (OtherActor :type Actor%20Object%20Reference) (OtherComp :type Primitive%20Component%20Object%20Reference) (OtherBodyIndex :type Integer))
  (Utilities|DoseImplementBpiSpLightRouteSpline OtherActor
    (:Then
      (Class|BPISpLightRouteSpline|RemoveRotateSpline(Message) OtherActor (Utilities|ResolveSoftReference (Variables|Default|GetSpline))))))

(fn ConstructionScript
  (スプライン|ResetBoxTransform))

(fn ResetBoxTransform
  (bind _spline (Variables|Default|GetSpline))
  (bind _validrangecapsule (Variables|Default|GetValidRangeCapsule))
  (bind _spline_2 (Variables|Default|GetSpline))
  (bind _validrangecapsule_2 (Variables|Default|GetValidRangeCapsule))
  (bind _splinelocationzbottomtop (LocalVariables|GetSplineLocationZBottomTop))
  (bind _boxstart (Variables|Default|GetBoxStart))
  (bind _boxend (Variables|Default|GetBoxEnd))
  (bind _returnvalue (Spline|GetNumberOfSplinePoints _spline))
  (bind _returnvalue_2 (Components|Box|GetScaledBoxExtent _boxstart))
  (bind _returnvalue_3 (Components|Box|GetScaledBoxExtent _boxend))
  (bind _returnvalue_4 (Spline|GetSplinePointAt _spline_2 0 "Local"))
  (bind (_x _y) (Math|Vector|BreakVector _returnvalue_2))
  (bind (_x_2 _y_2) (Math|Vector|BreakVector _returnvalue_3))
  (bind _returnvalue_5 (- _returnvalue 1))
  (bind _returnvalue_6 (Spline|GetSplinePointAt _spline _returnvalue_5 "Local"))
  (Utilities|FlowControl|Sequence
    (:then_0
      ;[1 1 1] 入り口・出口となる判定ボックスの座標を計算
      (Transformation|SetRelativeTransform (Variables|Default|GetBoxStart) (Math|Transform|MakeTransform (.position _returnvalue_4) (Math|Conversions|RotationFromXVector (.arrivetangent _returnvalue_4)) "1.000000,1.000000,1.000000") false true)
      (Transformation|SetRelativeTransform (Variables|Default|GetBoxEnd) (Math|Transform|MakeTransform (.position _returnvalue_6) (Math|Conversions|RotationFromXVector (* (.leavetangent _returnvalue_6) "-1.000000,-1.000000,1.000000")) (.scale _returnvalue_6)) false true)
      (Components|Box|SetBoxExtent (Variables|Default|GetBoxStart) (Variables|スプライン|GetBoxExtentStart) true)
      (Components|Box|SetBoxExtent (Variables|Default|GetBoxEnd) (Variables|スプライン|GetBoxExtentEnd) true))
    (:then_1
      (Utilities|FlowControl|Sequence
        (:then_0
          ;[1 1 1] スプラインの有効範囲を決定するカプセルの座標を計算
          (LocalVariables|SetCentroid "0, 0, 0")
          (for _index (range 0 (- (Spline|GetNumberOfSplinePoints (Variables|Default|GetSpline)) 1))
            (LocalVariables|SetCentroid (+ (LocalVariables|GetCentroid) (.Position (Utilities|Struct|BreakSplinePoint (Spline|GetSplinePointAt (Variables|Default|GetSpline) _index "Local")))))
            (Utilities|FlowControl|Sequence
              (:then_0
                (if (< (.Z (Math|Vector|BreakVector (.Position (Utilities|Struct|BreakSplinePoint (Spline|GetSplinePointAt (Variables|Default|GetSpline) _index "Local"))))) (Utilities|Array|Get(acopy) (LocalVariables|GetSplineLocationZBottomTop)))
                  (Utilities|Array|SetArrayElem (LocalVariables|GetSplineLocationZBottomTop) 0 (.Z (Math|Vector|BreakVector (.Position (Utilities|Struct|BreakSplinePoint (Spline|GetSplinePointAt (Variables|Default|GetSpline) _index "Local"))))) true) ; スプライトの下限座標を更新
                ))
              (:then_1
                (if (< (Utilities|Array|Get(acopy) (LocalVariables|GetSplineLocationZBottomTop) 1) (.Z (Math|Vector|BreakVector (.Position (Utilities|Struct|BreakSplinePoint (Spline|GetSplinePointAt (Variables|Default|GetSpline) _index "Local"))))))
                  (Utilities|Array|SetArrayElem (LocalVariables|GetSplineLocationZBottomTop) 1 (.Z (Math|Vector|BreakVector (.Position (Utilities|Struct|BreakSplinePoint (Spline|GetSplinePointAt (Variables|Default|GetSpline) _index "Local"))))) true) ; スプライトの上限座標を更新
                ))))
          (Transformation|SetRelativeLocation (Variables|Default|GetValidRangeCapsule) (/ (LocalVariables|GetCentroid) (Spline|GetNumberOfSplinePoints (Variables|Default|GetSpline))) false true) ; スプライトの重心に設定
        )
        (:then_1
          ;[1 1 1] スプラインの有効範囲となるカプセルの半径と高さを設定
          (LocalVariables|SetHorizontalDistanceMax 0.0)
          (for _index_2 (range 0 (- (Spline|GetNumberOfSplinePoints (Variables|Default|GetSpline)) 1))
            (if (< (LocalVariables|GetHorizontalDistanceMax) (Math|Vector|Distance2D(Vector) (.Position (Utilities|Struct|BreakSplinePoint (Spline|GetSplinePointAt (Variables|Default|GetSpline) _index_2 "Local"))) (Variables|/Script/Engine.SceneComponent|GetRelativeLocation (Variables|Default|GetValidRangeCapsule))))
              (LocalVariables|SetHorizontalDistanceMax (Math|Vector|Distance2D(Vector) (.Position (Utilities|Struct|BreakSplinePoint (Spline|GetSplinePointAt (Variables|Default|GetSpline) _index_2 "Local"))) (Variables|/Script/Engine.SceneComponent|GetRelativeLocation (Variables|Default|GetValidRangeCapsule))))
              (Components|Capsule|SetCapsuleHalfHeight _validrangecapsule_2 (+ (Math|Vector|Distance2D(Vector) (.Position (Utilities|Struct|BreakSplinePoint (Spline|GetSplinePointAt (Variables|Default|GetSpline) _index_2 "Local"))) (Variables|/Script/Engine.SceneComponent|GetRelativeLocation (Variables|Default|GetValidRangeCapsule))) (Math|Float|Max(Float) _x _y _x_2 _y_2) (.X (Math|Vector2D|BreakVector2D (Variables|スプライン|GetCupsulSizeBuffer)))) false) ; 範囲限度カプセルの半径設定のため先に設定
              (Components|Capsule|SetCapsuleRadius _validrangecapsule_2 (+ (Math|Vector|Distance2D(Vector) (.Position (Utilities|Struct|BreakSplinePoint (Spline|GetSplinePointAt (Variables|Default|GetSpline) _index_2 "Local"))) (Variables|/Script/Engine.SceneComponent|GetRelativeLocation (Variables|Default|GetValidRangeCapsule))) (Math|Float|Max(Float) _x _y _x_2 _y_2) (.X (Math|Vector2D|BreakVector2D (Variables|スプライン|GetCupsulSizeBuffer)))) false) ; 範囲限度カプセルの半径を設定
            ))
          (Components|Capsule|SetCapsuleHalfHeight _validrangecapsule (+ (Variables|/Script/Engine.CapsuleComponent|GetCapsuleHalfHeight _validrangecapsule) (* (Math|Float|Absolute(Float) (- (Utilities|Array|Get(acopy) _splinelocationzbottomtop) (Utilities|Array|Get(acopy) _splinelocationzbottomtop 1))) 0.5) (.Y (Math|Vector2D|BreakVector2D (Variables|スプライン|GetCupsulSizeBuffer))) (Math|Float|Max(Float) (.Z (Math|Vector|BreakVector (Components|Box|GetScaledBoxExtent (Variables|Default|GetBoxStart)))) (.Z (Math|Vector|BreakVector (Components|Box|GetScaledBoxExtent (Variables|Default|GetBoxEnd)))))) false) ; 範囲限度カプセルの高さを設定
        )))))