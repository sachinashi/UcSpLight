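; Sprite character base that receives custom SpLight lighting through a dynamic material instance driven by its light receiver component.
; Construction sets up the receiver and self light, then line-traces for an overlapping light source so lighting also applies in the editor.
; Capsule overlaps attach or release one external light, ignoring other characters' self lights, and follow its parameter-change event.
; Tick pushes contrast, strength, color and normal settings to the receiver.
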(event OnComponentBeginOverlap(CapsuleComponent)
  (params (OverlappedComponent :type Primitive%20Component%20Object%20Reference) (OtherActor :type Actor%20Object%20Reference) (OtherComp :type Primitive%20Component%20Object%20Reference) (OtherBodyIndex :type Integer) (bFromSweep :type Boolean) (SweepResult :type Hit%20Result%20Structure%20%28by%20ref%29))
  (bind _value (Utilities|SpLightCompClass))
  (bind _returnvalue (Actor|GetComponentbyClass OtherActor _value))
  ;[1 1 1] SpLight光源アクターの効果範囲に侵入した場合の処理
  (if (not (Class|GameplayStatics|ObjectIsA OtherActor (Utilities|SpLightCharClass))) ; 別キャラクターのセルフライトを候補から除外する
    (Utilities|IsValid _returnvalue
      (:Is%20Valid
        (bind _output_get (Variables|SpLight|SetUcSpLightComponent _returnvalue))
        (Default|CallOnBeginOverlapLight _output_get OtherComp self OverlappedComponent)
        (Default|SetLightSphere (Variables|コンポーネント|GetBP_SpLightReceiverComponent) (Variables|SpLight|GetUcSpLightComponent))
        (CallFunction|BindUcSpLightSphere (Variables|SpLight|GetUcSpLightComponent))))))

(event OnComponentEndOverlap(CapsuleComponent)
  (params (OverlappedComponent :type Primitive%20Component%20Object%20Reference) (OtherActor :type Actor%20Object%20Reference) (OtherComp :type Primitive%20Component%20Object%20Reference) (OtherBodyIndex :type Integer))
  (bind _value (Utilities|SpLightCompClass))
  (bind _returnvalue (Actor|GetComponentbyClass OtherActor _value))
  ;[1 1 1] SpLight光源アクターの効果範囲から離脱した場合の処理
  (if (not (Class|GameplayStatics|ObjectIsA OtherActor (Utilities|SpLightCharClass))) ; 別キャラクターのセルフライトを候補から除外する
    (Utilities|IsValid _returnvalue
      (:Is%20Valid
        (if (== _returnvalue (Variables|SpLight|GetUcSpLightComponent))
          (Default|CallOnEndOverlapLight (Variables|SpLight|GetUcSpLightComponent) OtherComp self OverlappedComponent)
          (Default|ResetLightSphere (Variables|コンポーネント|GetBP_SpLightReceiverComponent))
          (CallFunction|UnBindUcSpLightSphere (Variables|SpLight|GetUcSpLightComponent)))))))

(event Custom|ChangeSpLightSphere
  (params (Strength :type Float%20%28double-precision%29) (Hardness :type Float%20%28double-precision%29) (Radius :type Float%20%28double-precision%29) (WorldLocation :type Vector))
  ;[1 1 1] 光源の影響を処理する関数をバインド・アンバインドする
  (Default|SetLightSphere (Variables|コンポーネント|GetBP_SpLightReceiverComponent) (Variables|SpLight|GetUcSpLightComponent)))

(event Custom|BindUcSpLightSphere
  (params (SpLightComp :type BP%20Sp%20Light%20Component%20Object%20Reference) (Index :type Integer))
  ;[1 1 1] 光源の影響を処理する関数をバインド・アンバインドする
  (EventDispatchers|BindEventtoOnChangeLightParam SpLightComp (delegate Custom|ChangeSpLightSphere)))

(event Custom|UnBindUcSpLightSphere
  (params (SpLightComp :type BP%20Sp%20Light%20Component%20Object%20Reference) (Index :type Integer))
  ;[1 1 1] 光源の影響を処理する関数をバインド・アンバインドする
  (EventDispatchers|UnbindEventfromOnChangeLightParam SpLightComp (delegate Custom|ChangeSpLightSphere)))

(event EventBeginPlay)

(event Collision|EventActorBeginOverlap
  (params (OtherActor :type Actor%20Object%20Reference)))

(event EventTick
  (params (DeltaSeconds :type Float%20%28single-precision%29))
  (CallFunction|UpdateSpLightUtility))

(fn ConstructionScript
  (bind _self self)
  (bind _selflightcomponent (Variables|Default|GetSelfLightComponent))
  (bind _returnvalue (Transformation|GetActorLocation _self))
  (bind _returnvalue_2 (Rendering|Material|CreateDynamicMaterialInstance (Variables|Default|GetSprite) 0 0 "None" :!class /Script/Engine.PrimitiveComponent))
  (bind _output_get (Variables|SpLight|Material|SetAs%20Material%20Instance%20Dynamic _returnvalue_2))
  (Default|Init (Variables|コンポーネント|GetBP_SpLightReceiverComponent) _output_get (Variables|Default|GetSelfLightComponent))
  (Utilities|FlowControl|Sequence
    (:then_0
      ;[1 1 1] セルフSpLightの設定
      (Transformation|SetRelativeLocation _selflightcomponent (- (Variables|SpLight|Self|GetLightPosAdjust) (Variables|/Script/Engine.SceneComponent|GetRelativeLocation (Variables|Default|GetSprite))) false true)
      (Default|SetandUpdateLight _selflightcomponent (Variables|SpLight|Self|GetStrengthSelf) (Variables|SpLight|Self|GetHardnessSelf) (Variables|SpLight|Self|GetRadiusSelf) "0, 0, 0"))
    (:then_1
      ;[1 1 1] SpLight用光源アクターの初期設定
      (bind (_outhit _returnvalue_3) (Collision|LineTraceForObjects _returnvalue (+ _returnvalue "0.000000,0.000000,32.000000") (Utilities|Array|MakeArray (Utilities|Enum|LiteralenumEObjectTypeQuery "ObjectTypeQuery2")) false 0 "ForOneFrame"))
      (if _returnvalue_3
        (Utilities|IsValid (Actor|GetComponentbyClass (.HitActor (Collision|BreakHitResult _outhit)) "/UcSpLight/BluePrint/Component/BP_SpLightComponent.BP_SpLightComponent_C")
          (:Is%20Valid
            (bind _output_get_2 (Variables|SpLight|SetUcSpLightComponent (Actor|GetComponentbyClass (.HitActor (Collision|BreakHitResult _outhit)) "/UcSpLight/BluePrint/Component/BP_SpLightComponent.BP_SpLightComponent_C")))
            (Default|SetLightSphere (Variables|コンポーネント|GetBP_SpLightReceiverComponent) _output_get_2)
            (CallFunction|BindUcSpLightSphere (Variables|SpLight|GetUcSpLightComponent))))
        (else
          ;;[1 1 1] エディタ上で光源アクターと重なっていない場合、（干渉を防ぐため）超上空に光源を飛ばす
          (Default|ResetLightSphere (Variables|コンポーネント|GetBP_SpLightReceiverComponent))
          (Variables|SpLight|SetUcSpLightComponent 0))))
    (:then_2
      (CallFunction|UpdateSpLightUtility))))

(fn IsForwordforSprite
  (return (Utilities|Operators|EqualEqual (Transformation|GetActorForwardVector) (Math|Vector|MakeVector 0.0 1.0 0.0) 0.001)))

(fn UpdateSpLightUtility
  ;[1 1 1] SpLightの調整パラメーターを設定
  (Default|SetOverall (Variables|コンポーネント|GetBP_SpLightReceiverComponent) (Variables|SpLight|GetContrast) (Variables|SpLight|GetStrength))
  (Default|SetColorType (Variables|コンポーネント|GetBP_SpLightReceiverComponent) (Math|Conversions|ToFloat(Integer) (Variables|SpLight|GetColorType)))
  (Default|SetColorCorrection (Variables|コンポーネント|GetBP_SpLightReceiverComponent) (Variables|SpLight|GetColor%20Correction))
  (Default|SetNormal (Variables|コンポーネント|GetBP_SpLightReceiverComponent) (Variables|SpLight|GetNormal%20Strength) (Variables|SpLight|GetNormal%20Strength%20R) (Variables|SpLight|GetNormal%20Strength%20G) (Variables|SpLight|GetNormal%20Strength%20B)))