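; Level-wide settings Blueprint for the custom positional SpLight light sources, applying shared base values through the MPC_UcSpLightViewer material parameter collection.
; Its construction script calls SetLevelSpLight, which toggles editor display of all light sphere textures and writes base strength, contrast and per-channel normal strength.
; It also writes shadow compression controls as threshold, ratio and gain.
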(fn ConstructionScript
  (CallFunction|SetLevelSpLight))

(fn SetLevelSpLight
  (Utilities|FlowControl|Sequence
    (:then_0
      (Rendering|Material|SetScalarParameterValue "/UcSpLightV2/Art/SpLight/MPC_UcSpLightViewer.MPC_UcSpLightViewer" "ViewMaterial" (Math|Float|SelectFloat 0.0 1.0 (Variables|SpLight|GetHideAllSpLightSphere)) :!class /Script/Engine.KismetMaterialLibrary) ; エディタ上での、すべての自作光源テクスチャの表示非表示を変更する
    )
    (:then_1
      (Rendering|Material|SetScalarParameterValue "/UcSpLightV2/Art/SpLight/MPC_UcSpLightViewer.MPC_UcSpLightViewer" "LevelStrenghtBase" (* (Variables|SpLight|GetStrengthBase) 0.01) :!class /Script/Engine.KismetMaterialLibrary)
      (Rendering|Material|SetScalarParameterValue "/UcSpLightV2/Art/SpLight/MPC_UcSpLightViewer.MPC_UcSpLightViewer" "LevelContrastBase" (Variables|SpLight|GetContrastBase) :!class /Script/Engine.KismetMaterialLibrary)
      (Rendering|Material|SetVectorParameterValue "/UcSpLightV2/Art/SpLight/MPC_UcSpLightViewer.MPC_UcSpLightViewer" "LevelNormalStrengthBase" (Math|Color|MakeColor (Variables|SpLight|Normal|GetNormalStrengthRBase) (Variables|SpLight|Normal|GetNormalStrengthGBase) (Variables|SpLight|Normal|GetNormalStrengthBBase) (Variables|SpLight|Normal|GetNormalStrengthBase)) :!class /Script/Engine.KismetMaterialLibrary))
    (:then_2
      ;[1 1 1] 圧縮
      (Rendering|Material|SetScalarParameterValue "/UcSpLightV2/Art/SpLight/MPC_UcSpLightViewer.MPC_UcSpLightViewer" "LevelShadowThreshold" (Variables|SpLight|Compressor|GetShadowThreshold) :!class /Script/Engine.KismetMaterialLibrary)
      (Rendering|Material|SetScalarParameterValue "/UcSpLightV2/Art/SpLight/MPC_UcSpLightViewer.MPC_UcSpLightViewer" "LevelShadowRatio" (Variables|SpLight|Compressor|GetShadowRatio) :!class /Script/Engine.KismetMaterialLibrary)
      (Rendering|Material|SetScalarParameterValue "/UcSpLightV2/Art/SpLight/MPC_UcSpLightViewer.MPC_UcSpLightViewer" "LevelShadowGain" (Variables|SpLight|Compressor|GetShadowGain) :!class /Script/Engine.KismetMaterialLibrary))))