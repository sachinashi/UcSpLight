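; Placeable sphere light actor that applies its SpLightComponent lighting to SpLight actors within a box range.
; The construction script sizes the box and preview plane, pushes parameters to the component, and visualizes range, falloff, color and clipping through a dynamic material.
; It then calls setup through BPI_SpLightSetupfunc on overlapping actors and swaps its billboard to an error sprite when overlapping another sphere light.
; Tick repositions the optional in-game plane and refreshes its range.
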(event EventBeginPlay
  (Development|SetHiddeninGame (Variables|Default|GetLightInfluenceRangePlane) (not (Variables|SpLight|GetViewInGameLightInfluenceRange)) false))

(event EventTick
  (params (DeltaSeconds :type Float%20%28single-precision%29))
  (Transformation|SetRelativeLocation (Variables|Default|GetLightInfluenceRangePlane) (Variables|SpLight|GetOffset) false false)
  (if (not (Variables|/Script/Engine.SceneComponent|GetbHiddenInGame (Variables|Default|GetLightInfluenceRangePlane)))
    (SpLight|Material|UpdateSpLightMatRange)))

(fn ConstructionScript
  (bind _radius (Variables|SpLight|GetRadius))
  (bind _radius_2 (Variables|SpLight|GetRadius))
  (bind _shadoweffectivebox (Variables|Default|GetShadowEffectiveBox))
  (Utilities|FlowControl|Sequence
    (:then_0
      ;[1 1 1] 光源の適用範囲をまとめる
      (Variables|SpLight|SetLightRangeBox (Math|Vector|MakeVector (Variables|SpLight|GetLightDepth) (+ (Variables|SpLight|GetRadius) (Variables|SpLight|GetRangeBufferX)) (+ (Variables|SpLight|GetRadius) (Variables|SpLight|GetRangeBufferY))))
      (Rendering|Components|Sprite|SetSprite (Variables|Default|GetBillboard) (Utilities|LightTex)))
    (:then_1
      ;[1 1 1] 補助オブジェクトのサイズ変更
      (Components|Box|SetBoxExtent (Variables|Default|GetShadowEffectiveBox) (Variables|SpLight|GetLightRangeBox) false)
      (Transformation|SetRelativeScale3D (Variables|Default|GetLightInfluenceRangePlane) (Math|Vector|MakeVector (/ (Math|Float|SelectFloat _radius (.Y (Math|Vector|BreakVector (Variables|SpLight|GetLightRangeBox))) (< _radius (.Y (Math|Vector|BreakVector (Variables|SpLight|GetLightRangeBox))))) 5e+01) (/ (Math|Float|SelectFloat _radius_2 (.Z (Math|Vector|BreakVector (Variables|SpLight|GetLightRangeBox))) (< _radius_2 (.Z (Math|Vector|BreakVector (Variables|SpLight|GetLightRangeBox))))) 5e+01) (Math|Float|MakeLiteralFloat 1.0)))
      (Transformation|SetRelativeLocation (Variables|Default|GetLightInfluenceRangePlane) (Variables|SpLight|GetOffset) false false)
      ;[1 1 1] ライトコンポーネントの値を更新する
      (SpLight|UpdateLightComp))
    (:then_2
      ;[1 1 1] 視認用マテリアル設定
      (bind _returnvalue (Rendering|Material|CreateDynamicMaterialInstance (Variables|Default|GetLightInfluenceRangePlane) 0 0 "None" :!class /Script/Engine.PrimitiveComponent))
      (Variables|Default|SetMID_PlaneColor _returnvalue)
      (Utilities|FlowControl|Sequence
        (:then_0
          (SpLight|Material|UpdateSpLightMatBaseParam)
          (SpLight|Material|UpdateSpLightMatCenterParam))
        (:then_1
          (SpLight|Material|UpdateSpLightMatRange))
        (:then_2
          (SpLight|Material|UpdateSpLightMatColor))
        (:then_3
          (SpLight|Material|UpdateSpLightMatClipping))))
    (:then_3
      ;[1 1 1] 範囲内のSpLightアクターに配置光源を適用する
      (bind _outactors (Collision|ComponentOverlapActors _shadoweffectivebox (Transformation|GetWorldTransform _shadoweffectivebox) (Utilities|Array|MakeArray "ObjectTypeQuery1" "ObjectTypeQuery2" "ObjectTypeQuery3") "/Script/Engine.Actor"))
      (for _array_element _outactors
        (Utilities|FlowControl|Sequence
          (:then_0
            ;;[1 1 1] インターフェース経由で配置光源を初期化
            (if (Utilities|DoesObjectImplementInterface _array_element "/UcSpLightV2/BluePrint/Component/BPI_SpLightSetupfunc.BPI_SpLightSetupfunc_C")
              (Class|BPISpLightSetupfunc|SetupSphereLight(Message) _array_element)))
          (:then_1
            ;;[1 1 1] ライトの重複を検知（望ましくない）
            (if (Class|GameplayStatics|ObjectIsA _array_element "BP_SpLightSphere_C")
              (Rendering|Components|Sprite|SetSprite (Variables|Default|GetBillboard) (Utilities|LightTexErrer)))))))))

(fn GetLightParameters
  (return (Variables|SpLight|GetStrength) (Variables|SpLight|GetHardness) (Variables|SpLight|GetRadius) (Default|GetLightLocation (Variables|Default|GetSpLightComponent))))

(fn SetandUpdateLightComp
  (params (Strength :type Float%20%28double-precision%29) (Hardness :type Float%20%28double-precision%29) (Radius :type Float%20%28double-precision%29) (CenterStrength :type Float%20%28double-precision%29) (CenterHardness :type Float%20%28double-precision%29) (CenterRadius :type Float%20%28double-precision%29) (Offset :type Vector) (Clipping :type Linear%20Color%20Structure))
  (Default|SetandUpdateLight (Variables|Default|GetSpLightComponent) Strength Hardness Radius CenterStrength CenterHardness CenterRadius Offset Clipping))

(fn UpdateLightComp
  (SpLight|SetandUpdateLightComp (Variables|SpLight|GetStrength) (Variables|SpLight|GetHardness) (Variables|SpLight|GetRadius) (Variables|SpLight|GetCenterStrength) (Variables|SpLight|GetCenterHardness) (Variables|SpLight|GetCenterRadius) (Variables|SpLight|GetOffset) (Utilities|CastClippingtoColor)))

(fn UpdateSpLightMatRange
  (bind _mid_planecolor (Variables|Default|GetMID_PlaneColor))
  (bind _offset (Variables|SpLight|GetOffset))
  (bind _lightrangebox (Variables|SpLight|GetLightRangeBox))
  (bind _offset_2 (Variables|SpLight|GetOffset))
  (bind _lightrangebox_2 (Variables|SpLight|GetLightRangeBox))
  (bind _mid_planecolor_2 (Variables|Default|GetMID_PlaneColor))
  (bind _returnvalue (* _lightrangebox 1.0))
  (bind _returnvalue_2 (* _lightrangebox_2 -1.0))
  (bind _returnvalue_3 (- _returnvalue_2 _offset))
  (bind _returnvalue_4 (- _returnvalue _offset_2))
  (bind (_x _y _z) (Math|Vector|BreakVector _returnvalue_4))
  (bind (_x_2 _y_2 _z_2) (Math|Vector|BreakVector _returnvalue_3))
  (Utilities|FlowControl|Sequence
    (:then_0
      ;[1 1 1] 光源の適用範囲を可視化する情報をマテリアルに送る
      (Rendering|Material|SetScalarParameterValue _mid_planecolor "RangeXLeft" _y_2 :!class /Script/Engine.MaterialInstanceDynamic)
      (Rendering|Material|SetScalarParameterValue _mid_planecolor "RangeYBottom" _z_2 :!class /Script/Engine.MaterialInstanceDynamic)
      (Rendering|Material|SetScalarParameterValue _mid_planecolor "RangeXRIght" _y :!class /Script/Engine.MaterialInstanceDynamic)
      (Rendering|Material|SetScalarParameterValue _mid_planecolor "RangeYTop" _z :!class /Script/Engine.MaterialInstanceDynamic))
    (:then_1
      ;[1 1 1] 有効・非有効範囲の透明度をマテリアルに送る
      (Rendering|Material|SetScalarParameterValue _mid_planecolor_2 "OpacityRangeIn" (Variables|SpLight|GetOpacityRangeIn) :!class /Script/Engine.MaterialInstanceDynamic)
      (Rendering|Material|SetScalarParameterValue _mid_planecolor_2 "OpacityRangeOut" (Variables|SpLight|GetOpacityRangeOut) :!class /Script/Engine.MaterialInstanceDynamic))))

(fn UpdateSpLightMatBaseParam
  (bind _mid_planecolor (Variables|Default|GetMID_PlaneColor))
  (Rendering|Material|SetScalarParameterValue _mid_planecolor "Strength" (* (Variables|SpLight|GetStrength) 0.01) :!class /Script/Engine.MaterialInstanceDynamic)
  (Rendering|Material|SetScalarParameterValue _mid_planecolor "Radius" (Variables|SpLight|GetRadius) :!class /Script/Engine.MaterialInstanceDynamic)
  (Rendering|Material|SetScalarParameterValue _mid_planecolor "Hardness" (Variables|SpLight|GetHardness) :!class /Script/Engine.MaterialInstanceDynamic))

(fn UpdateSpLightMatCenterParam
  (bind _mid_planecolor (Variables|Default|GetMID_PlaneColor))
  (Rendering|Material|SetScalarParameterValue _mid_planecolor "CenterStrength" (* (Variables|SpLight|GetCenterStrength) 0.01) :!class /Script/Engine.MaterialInstanceDynamic)
  (Rendering|Material|SetScalarParameterValue _mid_planecolor "CenterRadiusPercent" (* (Variables|SpLight|GetCenterRadius) 0.01) :!class /Script/Engine.MaterialInstanceDynamic)
  (Rendering|Material|SetScalarParameterValue _mid_planecolor "CenterHardness" (Variables|SpLight|GetCenterHardness) :!class /Script/Engine.MaterialInstanceDynamic))

(fn UpdateSpLightMatColor
  (bind _mid_planecolor (Variables|Default|GetMID_PlaneColor))
  (bind _lightrangein (Variables|SpLight|GetLightRangeIn))
  (Rendering|Material|SetVectorParameterValue _mid_planecolor "ColorRangeIn" (Math|Color|SelectColor (- "(R=1.000000,G=1.000000,B=1.000000,A=1.000000)" _lightrangein) _lightrangein (< (Variables|SpLight|GetStrength) 0.0)) :!class /Script/Engine.MaterialInstanceDynamic)
  (Rendering|Material|SetVectorParameterValue _mid_planecolor "ColorRangeOut" (Variables|SpLight|GetLightRangeOut) :!class /Script/Engine.MaterialInstanceDynamic))

(fn UpdateSpLightMatClipping
  (bind _linearcolor (Utilities|CastClippingtoColor))
  (bind _lightrangebox (Variables|SpLight|GetLightRangeBox))
  (bind _lightrangebox_2 (Variables|SpLight|GetLightRangeBox))
  (bind _z (Math|Vector|BreakVector _lightrangebox))
  (bind (_r _g _b _a) (Math|Color|BreakColor _linearcolor))
  (bind _y (Math|Vector|BreakVector _lightrangebox_2))
  ;[1 1 1] クリッピングの比率を調整
  (LocalVariables|SetScaleClippingX (Math|Float|SelectFloat (/ (Variables|SpLight|GetRadius) _y) 1.0 (< _y (Variables|SpLight|GetRadius))))
  (LocalVariables|SetScaleClippingY (Math|Float|SelectFloat (/ (Variables|SpLight|GetRadius) _z) 1.0 (< _z (Variables|SpLight|GetRadius))))
  (Rendering|Material|SetVectorParameterValue (Variables|Default|GetMID_PlaneColor) "Clipping" (Math|Color|MakeColor (* _r (LocalVariables|GetScaleClippingX)) (* _g (LocalVariables|GetScaleClippingY)) (* _b (LocalVariables|GetScaleClippingX)) (* _a (LocalVariables|GetScaleClippingY))) :!class /Script/Engine.MaterialInstanceDynamic))